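; BP_MeasuringCube is an editor-configurable wireframe box sized in centimeters, with a settable emissive color.
; The construction script creates a dynamic material instance for the WireBox behind a DoOnce and applies the EmissiveColor to its front emissive parameter.
; It multiplies the box's current world scale on each axis by that axis's centimeter value divided by 100.
; The event graph contains no active logic.
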(event EventBeginPlay)

(event Collision|EventActorBeginOverlap
  (params (OtherActor :type Actor%20Object%20Reference)))

(event EventTick
  (params (DeltaSeconds :type Float%20%28single-precision%29)))

(fn ConstructionScript
  (bind _wirebox (Variables|Default|GetWireBox))
  (bind _wirebox_2 (Variables|Default|GetWireBox))
  (bind _returnvalue (Transformation|GetWorldScale _wirebox))
  (Utilities|FlowControl|Sequence
    (:then_0
      (Utilities|FlowControl|DoOnce false
        (:Completed
          (bind _returnvalue_2 (Rendering|Material|CreateDynamicMaterialInstance _wirebox_2 0 (Rendering|Material|GetMaterial _wirebox_2 0) "None" :!class /Script/Engine.PrimitiveComponent))
          (Rendering|Material|GetVectorParameterValue _returnvalue_2 "EmissiveColorFront" :!class /Script/Engine.MaterialInstanceDynamic)
          (Rendering|Material|SetMaterial _wirebox_2 0 _returnvalue_2))))
    (:then_1
      (Transformation|SetWorldScale3D _wirebox (Math|Vector|MakeVector (* (.x _returnvalue) (/ (Variables|Default|GetCentimeters_X) 1e+02)) (* (.y _returnvalue) (/ (Variables|Default|GetCentimeters_Y) 1e+02)) (* (.z _returnvalue) (/ (Variables|Default|GetCentimeters_Z) 1e+02))))
      (Rendering|Material|SetVectorParameterValue _returnvalue_2 "EmissiveColorFront" (Variables|Default|GetEmissiveColor) :!class /Script/Engine.MaterialInstanceDynamic))))